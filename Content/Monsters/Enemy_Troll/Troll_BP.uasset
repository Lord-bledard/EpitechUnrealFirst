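; Troll enemy that targets the player through AI perception, attacks with a sword, and reports its spawn and death to the game mode's enemy counters.
; A forward sphere trace that finds the player triggers the attack montage through server-to-multicast events.
; A looping timer line-traces between two arrows to apply sword damage until stopped.
; A proximity sphere toggles the floating health bar, which damage updates until death.
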(event `self.AIPerception.OnTargetPerceptionUpdated`
  (params (Actor :type "Actor Object Reference") (Stimulus :type "AIStimulus Structure"))
  (if (`self.ActorHasTag` Actor "Player")
    (`BlackboardComponent.SetValueAsObject` (`AIBlueprintHelperLibrary.GetBlackboard` (`AIBlueprintHelperLibrary.GetAIController` self)) "Target" Actor)))

(event `S_Server`
  (`self.M_Multi`))

(event `attackplayer`
  (bind _returnvalue (`self.K2_GetActorLocation`))
  (bind (_outhit _returnvalue_2) (`KismetSystemLibrary.SphereTraceSingleForObjects` :`Start` _returnvalue :`End` (+ _returnvalue (* (`KismetMathLibrary.GetForwardVector` (`self.K2_GetActorRotation`)) 250.0)) :`Radius` 120.0 :`ObjectTypes` (`|MakeArray` "ObjectTypeQuery3" :!type "EObjectTypeQuery Enum") :`DrawDebugType` "ForOneFrame"))
  (if _returnvalue_2
    (if (`self.ActorHasTag` (`.HitActor` (`GameplayStatics.BreakHitResult` _outhit)) "Player")
      (`self.S_Server`))))

(event `M_Multi`
  (`KismetSystemLibrary.PrintString` "Hello")
  (`self.PlayAnimMontage` "/Game/Enemy/Enemy_Troll/Enemy_Troll_Poison_Animation/Troll_Attack.Troll_Attack"))

(event `self.ReceiveBeginPlay`
  (bind _asbp_first_person_game_mode (cast `/Game/FirstPerson/Blueprints/BP_FirstPersonGameMode` (`GameplayStatics.GetGameMode`)))
  (`/Engine/EditorBlueprintResources/StandardMacros.IncrementInt` (`/Game/FirstPerson/Blueprints/BP_FirstPersonGameMode.EnnemyAlive` _asbp_first_person_game_mode)
    (:`  `
      (`SceneComponent.SetVisibility` (`self.HealthBar`) false false))))

(event `triggersword`
  (bind _returnvalue (`KismetSystemLibrary.K2_SetTimerDelegate` (delegate `swordlinetrace`) 0.01 true))
  (set `self.triggerswordevent` _returnvalue))

(event `swordlinetrace`
  (bind _outhit (`KismetSystemLibrary.LineTraceSingle` :`Start` (`SceneComponent.GetSocketLocation` (`self.Arrow1`) "start") :`End` (`SceneComponent.GetSocketLocation` (`self.Arrow2`) "end") :`TraceChannel` "TraceTypeQuery2" :`DrawDebugType` "ForDuration"))
  (bind (_bblockinghit _binitialoverlap _time _distance _location _impactpoint _normal _impactnormal _physmat _hitactor) (`GameplayStatics.BreakHitResult` _outhit))
  (if (`self.ActorHasTag` _hitactor "Player")
    (`GameplayStatics.ApplyDamage` _hitactor 20.0)))

(event `stoptrigger`
  (`KismetSystemLibrary.K2_ClearAndInvalidateTimerHandle` (`self.triggerswordevent`)))

(event `force`
  (bind _returnvalue (`|CreateWidget` "/Game/HUD/FloatingHealthBar.FloatingHealthBar_C" :!label _label))
  (`WidgetComponent.SetWidget` (`self.HealthBar`) _returnvalue)
  (set `/Game/HUD/FloatingHealthBar.Name` (`self.MonsterName`) _returnvalue)
  (set `/Game/HUD/FloatingHealthBar.Level` (`self.Level`) _returnvalue)
  (set `/Game/HUD/FloatingHealthBar.MaxHealth` (`self.MaxHealth`) _returnvalue)
  (set `/Game/HUD/FloatingHealthBar.Health` (`self.Health`) _returnvalue)
  (set `self.FloatingHealthBar` _returnvalue)
  (`SceneComponent.SetVisibility` (`self.HealthBar`) true true))

(event `self.Sphere_floatbar.OnComponentBeginOverlap`
  (params (OverlappedComponent :type "PrimitiveComponent Object Reference") (OtherActor :type "Actor Object Reference") (OtherComp :type "PrimitiveComponent Object Reference") (OtherBodyIndex :type Integer) (bFromSweep :type Boolean) (SweepResult :type "HitResult Structure (by ref)"))
  (if (`self.ActorHasTag` OtherActor "Player")
    (goto _label)))

(event `self.ReceiveAnyDamage`
  (params (Damage :type "Float (single-precision)") (DamageType :type "DamageType Object Reference") (InstigatedBy :type "Controller Object Reference") (DamageCauser :type "Actor Object Reference"))
  (bind _output_get (set `self.Health` (`KismetMathLibrary.FClamp` (- (`self.Health`) Damage) 0.0 (`self.MaxHealth`))))
  (set `/Game/HUD/FloatingHealthBar.Health` _output_get (`self.FloatingHealthBar`))
  (if (== (`self.Health`) 0.0)
    (`self.K2_DestroyActor`)
    (bind _asbp_first_person_game_mode (cast `/Game/FirstPerson/Blueprints/BP_FirstPersonGameMode` (`GameplayStatics.GetGameMode`)))
    (`/Engine/EditorBlueprintResources/StandardMacros.DecrementInt` (`/Game/FirstPerson/Blueprints/BP_FirstPersonGameMode.EnnemyAlive` _asbp_first_person_game_mode)
      (:`  `
        (`/Engine/EditorBlueprintResources/StandardMacros.IncrementInt` (`/Game/FirstPerson/Blueprints/BP_FirstPersonGameMode.EnnemyKill` _asbp_first_person_game_mode)
          (:`  `
            (`/Game/FirstPerson/Blueprints/BP_FirstPersonGameMode.CheckEnnemyLeft` _asbp_first_person_game_mode)))))
    (else
      (set `self.Hurt` true)
      (`KismetSystemLibrary.Delay` 0.1)
      (set `self.Hurt` false))))

(event `self.Sphere_floatbar.OnComponentEndOverlap`
  (params (OverlappedComponent :type "PrimitiveComponent Object Reference") (OtherActor :type "Actor Object Reference") (OtherComp :type "PrimitiveComponent Object Reference") (OtherBodyIndex :type Integer))
  (if (`self.ActorHasTag` OtherActor "Player")
    (`SceneComponent.SetVisibility` (`self.HealthBar`) false false)))

(fn `UserConstructionScript`)